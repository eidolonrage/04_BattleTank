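; Tank Blueprint that handles the player's aiming camera; the graph contains only camera input, with no movement or firing logic.
; AimAzimuth yaws the AzimuthGimbal, while AimElevation pitches the SpringArm, with InvertYLook choosing the sign.
; After either axis input, the gimbal's world pitch and roll are zeroed and its yaw kept, so the camera's rotation plane stays flat regardless of terrain.
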(event `InputAxis|AimAzimuth`
  (params (AxisValue :type "Float (single-precision)"))
  (bind _azimuth_gimbal (`self.Azimuth Gimbal`))
  (bind (_returnvalue_roll _returnvalue_pitch _returnvalue_yaw) (`KismetMathLibrary.BreakRotator` (`SceneComponent.K2_GetComponentRotation` _azimuth_gimbal)))
  ;[1 1 1] Camera Input Bindings
  (`SceneComponent.K2_AddLocalRotation` (`self.Azimuth Gimbal`) (`KismetMathLibrary.MakeRotator` 0.0 0.0 AxisValue) false false)
  ;;[1 1 1] Maintain a flat rotation plane regardless of terrain
  (`SceneComponent.K2_SetWorldRotation` _azimuth_gimbal (`KismetMathLibrary.MakeRotator` 0.0 0.0 _returnvalue_yaw) false false :!label _label))

(event `InputAxis|AimElevation`
  (params (AxisValue :type "Float (single-precision)"))
  (bind _springarm (`self.SpringArm`))
  ;[1 1 1] Camera Input Bindings
  (if (`self.invertYLook`)
    (`SceneComponent.K2_AddLocalRotation` _springarm (`KismetMathLibrary.MakeRotator` 0.0 AxisValue) false false)
    (goto _label)
    (else
      (`SceneComponent.K2_AddLocalRotation` _springarm (`KismetMathLibrary.MakeRotator` 0.0 (* AxisValue -1.0)) false false)
      (goto _label))))

(fn `UserConstructionScript`)